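; World border actor that keeps the player inside the play area using three border components.
; The BorderSwitch macro routes player overlap events by component, each printing a debug name.
; Leaving the second border starts a HUD warning and re-entering ends it.
; Leaving the third teleports the player to the closest point on the first, with height set by a vertical line trace that ignores instanced foliage.
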(event Custom|OnComponentBeginOverlap
  (params (OverlappedComponent :type Primitive%20Component%20Object%20Reference) (OtherActor :type Actor%20Object%20Reference) (OtherComp :type Primitive%20Component%20Object%20Reference) (OtherBodyIndex :type Integer) (bFromSweep :type Boolean) (SweepResult :type Hit%20Result%20Structure%20%28by%20ref%29))
  (Utilities|Casting|CastToBP_PlayerCharacter OtherActor)
  (Utilities|BorderSwitch OverlappedComponent
    (:1st%20Border
      (Development|PrintString (Utilities|GetDisplayName (Variables|Default|Get1st%20Border))))
    (:2nd%20Border
      (Development|PrintString (Utilities|GetDisplayName (Variables|Default|Get2nd%20Border)))
      (bind _asbp_player_hud (Utilities|Casting|CastToBP_PlayerHUD (HUD|GetHUD (Game|GetPlayerController 0))))
      (Default|BorderWarningEnd _asbp_player_hud))
    (:3rd%20Border
      (Development|PrintString (Utilities|GetDisplayName (Variables|Default|Get3rd%20border))))
    (:Default
      (Development|PrintString "Error!"))))

(event Custom|OnComponentEndOverlap
  (params (OverlappedComponent :type Primitive%20Component%20Object%20Reference) (OtherActor :type Actor%20Object%20Reference) (OtherComp :type Primitive%20Component%20Object%20Reference) (OtherBodyIndex :type Integer))
  (bind _returnvalue (Transformation|GetActorLocation OtherActor))
  (bind _1st_border (Variables|Default|Get1st%20Border))
  (bind _outpointonbody (Collision|GetClosestPointonCollision _1st_border _returnvalue "None"))
  (Utilities|Casting|CastToBP_PlayerCharacter OtherActor)
  (Utilities|BorderSwitch OverlappedComponent
    (:1st%20Border
      (Development|PrintString (Utilities|GetDisplayName (Variables|Default|Get1st%20Border))))
    (:2nd%20Border
      (Development|PrintString (Utilities|GetDisplayName (Variables|Default|Get2nd%20Border)))
      (bind _asbp_player_hud (Utilities|Casting|CastToBP_PlayerHUD (HUD|GetHUD (Game|GetPlayerController 0))))
      (Default|BorderWarningStart _asbp_player_hud))
    (:3rd%20Border
      (Development|PrintString (Utilities|GetDisplayName (Variables|Default|Get3rd%20border)))
      (bind _outactors (Actor|GetAllActorsOfClass "/Script/Foliage.InstancedFoliageActor"))
      (bind _outhit (Collision|LineTraceForObjects (Math|Vector|MakeVector (.x _outpointonbody) (.y _outpointonbody) 1e+06) (Math|Vector|MakeVector 0.0 0.0 -1e+06) (Utilities|Array|MakeArray "ObjectTypeQuery1") false _outactors "None"))
      (Transformation|SetActorLocation OtherActor (Math|Vector|MakeVector (.x (.Location (Collision|BreakHitResult _outhit))) (.y (.Location (Collision|BreakHitResult _outhit))) (+ (.z (.Location (Collision|BreakHitResult _outhit))) 9e+01)) false true))
    (:Default
      (Development|PrintString "Error!"))))

(event EventBeginPlay
  (bind _1st_border (Variables|Default|Get1st%20Border))
  (Utilities|FlowControl|Sequence
    (:then_0
      (Collision|AssignOnComponentBeginOverlap _1st_border (delegate Custom|OnComponentBeginOverlap)))
    (:then_1
      (Collision|AssignOnComponentEndOverlap _1st_border (delegate Custom|OnComponentEndOverlap)))))

(fn ConstructionScript)