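; DamageBox is a demo-room hazard actor that deals continuous environmental damage to an actor overlapping it.
; Begin and end overlap set a flag and store the latest actor, with no check that it is the player.
; While the flag is set, Tick applies DamagePerSecond scaled by delta time to that single stored actor.
; BeginPlay caches the player character, but the damage logic never uses that reference.
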(event Collision|EventActorBeginOverlap
  (params (OtherActor :type Actor%20Object%20Reference))
  (Variables|Default|SetOverlappingWithPlayer true)
  (Variables|Default|SetdamagedActor OtherActor))

(event Collision|EventActorEndOverlap
  (params (OtherActor :type Actor%20Object%20Reference))
  (Variables|Default|SetOverlappingWithPlayer false)
  (Variables|Default|SetdamagedActor OtherActor))

(event EventTick
  (params (DeltaSeconds :type Float%20%28single-precision%29))
  (if (Variables|Default|GetOverlappingWithPlayer)
    (Game|Damage|ApplyDamage (Variables|Default|GetdamagedActor) (* (Utilities|Time|GetWorldDeltaSeconds) (Variables|Default|GetDamagePerSecond)) 0 self "/Engine/EngineDamageTypes/DmgTypeBP_Environmental.DmgTypeBP_Environmental_C")))

(event EventBeginPlay
  (bind _asbp_player_character (Utilities|Casting|CastToBP_PlayerCharacter (Game|GetPlayerCharacter 0)))
  (Variables|Default|SetCharacterRef _asbp_player_character))

(fn ConstructionScript)