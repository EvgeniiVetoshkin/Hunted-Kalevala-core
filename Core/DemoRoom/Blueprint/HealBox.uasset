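; HealBox is a demo room actor that continuously heals the player character while its overlap flag is set.
; BeginPlay caches player 0's BP_PlayerCharacter, and the begin and end overlap events set or clear the flag without checking which actor overlaps.
; While the flag is set, Tick calls Heal on the cached character with HealPerSecond scaled by world delta time.
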(event Collision|EventActorBeginOverlap
  (params (OtherActor :type Actor%20Object%20Reference))
  (Variables|Default|SetOverlappingWithPlayer true))

(event Collision|EventActorEndOverlap
  (params (OtherActor :type Actor%20Object%20Reference))
  (Variables|Default|SetOverlappingWithPlayer false))

(event EventTick
  (params (DeltaSeconds :type Float%20%28single-precision%29))
  (if (Variables|Default|GetOverlappingWithPlayer)
    (Default|Heal (Variables|Default|GetCharacterRef) (* (Utilities|Time|GetWorldDeltaSeconds) (Variables|Default|GetHealPerSecond)))))

(event EventBeginPlay
  (bind _asbp_player_character (Utilities|Casting|CastToBP_PlayerCharacter (Game|GetPlayerCharacter 0)))
  (Variables|Default|SetCharacterRef _asbp_player_character))

(fn ConstructionScript)